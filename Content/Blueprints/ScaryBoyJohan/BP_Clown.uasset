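; BP_Clown is a scary clown enemy that plays a spawn sound and keeps turning toward the player's camera on a looping timer.
; When looked at, a jump-scare spawn laughs and vanishes after a brief delay.
; Otherwise it plays a stepping animation, then explodes in Niagara effects with a laugh and destroys itself.
; Player overlap with the capsule only prints a death message.
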(event `/Game/Blueprints/ScaryBoyJohan/INT_Clown.PlayerLooksAtDemon`
  (if (`self.SpawnedWithJumpScare`)
    (`KismetSystemLibrary.Delay` 0.2)
    ;[1 0.7979 0] laughing sound
    (`GameplayStatics.PlaySoundAtLocation` null (`self.K2_GetActorLocation`) (struct) 1.0 1.0 0.0 null null null null)
    (`self.K2_DestroyActor`)
    (else
      (`/Game/Blueprints/ScaryBoyJohan/INT_Clown.OneStep`))))

(event `/Game/Blueprints/ScaryBoyJohan/INT_Clown.OneStep`
  (bind _returnvalue (`SceneComponent.K2_GetComponentLocation` (`self.Mesh`)))
  ;[1 1 1] step closer to player
  (`SkeletalMeshComponent.PlayAnimation` (`self.Mesh`) "/Game/Blueprints/ScaryBoyJohan/Animations/Scary_Clown_Stopping__1_.Scary_Clown_Stopping__1_" true)
  (`KismetSystemLibrary.Delay` 1.33)
  (`NiagaraFunctionLibrary.SpawnSystemAtLocation` "/Niagara/DefaultAssets/Templates/Systems/SimpleExplosion.SimpleExplosion" _returnvalue)
  ;;[1 0.7979 0] laughing sound
  (`GameplayStatics.PlaySoundAtLocation` null _returnvalue (struct) 1.0 1.0 0.0 null null null null)
  (`self.K2_DestroyActor`))

(event `self.Capsule.OnComponentBeginOverlap`
  (params (OverlappedComponent :type "PrimitiveComponent Object Reference") (OtherActor :type "Actor Object Reference") (OtherComp :type "PrimitiveComponent Object Reference") (OtherBodyIndex :type Integer) (bFromSweep :type Boolean) (SweepResult :type "HitResult Structure (by ref)"))
  ;[1 0.4474 0.4374] Death
  (if (== OtherActor (`GameplayStatics.GetPlayerCharacter` 0))
    (`KismetSystemLibrary.PrintString` "You just died mate" true true (struct :`R` 1.0 :`B` 0.053326 :`A` 1.0))))

(event `self.ReceiveBeginPlay`
  ;[1 1 1] constatly rotate to player
  (`GameplayStatics.PlaySoundAtLocation` "/Game/Sounds/CloundSounds/ClownSpawn.ClownSpawn" (`self.K2_GetActorLocation`) (struct) 1.0 1.0 0.0 null null null null)
  (`KismetSystemLibrary.K2_SetTimerDelegate` (delegate `LokAt Player`) 0.1 true))

(event `LokAt Player`
  (bind (_returnvalue_roll _returnvalue_pitch _returnvalue_yaw) (`KismetMathLibrary.BreakRotator` (`KismetMathLibrary.FindLookAtRotation` (`SceneComponent.K2_GetComponentLocation` (`self.Mesh`)) (`PlayerCameraManager.GetCameraLocation` (`GameplayStatics.GetPlayerCameraManager` 0)))))
  ;[1 1 1] constatly rotate to player
  (`self.K2_SetActorRotation` (`KismetMathLibrary.MakeRotator` _returnvalue_roll 0.0 _returnvalue_yaw)))

(fn `UserConstructionScript`)