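; BP_Jumpscare is a one-shot trigger volume that plays a jumpscare when the player enters its bounding box.
; A JumpscareType setting selects a door slam followed by a delayed clown spawn, a window slam sound, or an immediate clown spawn.
; The door slam is sent to a referenced DoorActor, while sounds and BP_Clown spawns use the SpawnPoint component, with clowns flagged as jumpscare spawns.
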(event `self.BoundingBox.OnComponentBeginOverlap`
  (params (OverlappedComponent :type "PrimitiveComponent Object Reference") (OtherActor :type "Actor Object Reference") (OtherComp :type "PrimitiveComponent Object Reference") (OtherBodyIndex :type Integer) (bFromSweep :type Boolean) (SweepResult :type "HitResult Structure (by ref)"))
  (bind (_returnvalue_location _returnvalue_rotation) (`KismetMathLibrary.BreakTransform` (`SceneComponent.K2_GetComponentToWorld` (`self.SpawnPoint`))))
  (bind (_returnvalue_location_2 _returnvalue_rotation_2) (`KismetMathLibrary.BreakTransform` (`SceneComponent.K2_GetComponentToWorld` (`self.SpawnPoint`))))
  (if (== OtherActor (`GameplayStatics.GetPlayerCharacter` 0))
    (`/Engine/EditorBlueprintResources/StandardMacros.DoOnce` false
      (:`Completed`
        (switch `/Game/Blueprints/E_Jumpscare` (`self.JumpscareType`)
          (:`NewEnumerator0`
            ;[1 1 1] doorslam + clown spawn
            ;;[1 1 1] close door
            (message `/Game/Blueprints/BPI_Interact.DoorSlam` (`self.DoorActor`))
            (`KismetSystemLibrary.Delay` 2.3)
            (`|SpawnActorFromClass` "/Game/Blueprints/ScaryBoyJohan/BP_Clown.BP_Clown_C" (`KismetMathLibrary.MakeTransform` (+ _returnvalue_location_2 (0.0 0.0 100.0)) _returnvalue_rotation_2) "AlwaysSpawn" "OverrideRootScale" null true null))
          (:`NewEnumerator1`
            ;[1 1 1] windowsound
            (`GameplayStatics.PlaySoundAtLocation` null (`SceneComponent.K2_GetComponentLocation` (`self.SpawnPoint`)) (struct) 1.0 1.0 0.0 null null null null))
          (:`NewEnumerator2`
            ;[1 1 1] clown spawn
            (`|SpawnActorFromClass` "/Game/Blueprints/ScaryBoyJohan/BP_Clown.BP_Clown_C" (`KismetMathLibrary.MakeTransform` (+ _returnvalue_location (0.0 0.0 100.0)) _returnvalue_rotation) "AlwaysSpawn" "OverrideRootScale" null true null)))))))

(fn `UserConstructionScript`)