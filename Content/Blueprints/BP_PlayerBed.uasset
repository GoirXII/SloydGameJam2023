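; BP_PlayerBed is the player's bed, acting as the delivery point for a quest to place a teddy.
; Overlapping the QuestDelivery component with a "Teddy"-tagged player sets the character's IsOverlapping flag and shows a "Place Teddy" HUD prompt, hidden on end overlap.
; Interact rechecks the flag and tag, reveals the bed's Teddy component and sends a quest-completed message to the player character.
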(event `self.ReceiveBeginPlay`
  (bind _asbp_sleep_deprived_dude (cast `/Game/Blueprints/BP_SleepDeprivedDude` (`GameplayStatics.GetPlayerCharacter` 0)))
  (set `self. BP Sleep Deprived Dude` _asbp_sleep_deprived_dude))

(event `self.QuestDelivery.OnComponentBeginOverlap`
  (params (OverlappedComponent :type "PrimitiveComponent Object Reference") (OtherActor :type "Actor Object Reference") (OtherComp :type "PrimitiveComponent Object Reference") (OtherBodyIndex :type Integer) (bFromSweep :type Boolean) (SweepResult :type "HitResult Structure (by ref)"))
  (bind __bp_sleep_deprived_dude (`self. BP Sleep Deprived Dude`))
  (bind _wb_hud (`/Game/Blueprints/BP_SleepDeprivedDude.WB_HUD` __bp_sleep_deprived_dude))
  (if (== OtherActor __bp_sleep_deprived_dude)
    (if (`self.ActorHasTag` (`GameplayStatics.GetPlayerCharacter` 0) "Teddy")
      (set `/Game/Blueprints/BP_SleepDeprivedDude.IsOverlapping` true __bp_sleep_deprived_dude)
      (`TextBlock.SetText` (`/Game/Widgets/WB_HUD.Prompt_Text` _wb_hud) "Place")
      (`TextBlock.SetText` (`/Game/Widgets/WB_HUD.Item_Text` _wb_hud) "Teddy")
      (`Widget.SetVisibility` (`/Game/Widgets/WB_HUD.PickUp_VB` _wb_hud) "SelfHitTestInvisible"))))

(event `self.QuestDelivery.OnComponentEndOverlap`
  (params (OverlappedComponent :type "PrimitiveComponent Object Reference") (OtherActor :type "Actor Object Reference") (OtherComp :type "PrimitiveComponent Object Reference") (OtherBodyIndex :type Integer))
  (bind __bp_sleep_deprived_dude (`self. BP Sleep Deprived Dude`))
  (set `/Game/Blueprints/BP_SleepDeprivedDude.IsOverlapping` false __bp_sleep_deprived_dude)
  (`Widget.SetVisibility` (`/Game/Widgets/WB_HUD.PickUp_VB` (`/Game/Blueprints/BP_SleepDeprivedDude.WB_HUD` __bp_sleep_deprived_dude)) "Collapsed"))

(event `/Game/Blueprints/BPI_Interact.Interact`
  (bind _returnvalue (`GameplayStatics.GetPlayerCharacter` 0))
  (if (`/Game/Blueprints/BP_SleepDeprivedDude.IsOverlapping` (`self. BP Sleep Deprived Dude`))
    (if (`self.ActorHasTag` _returnvalue "Teddy")
      (`SceneComponent.SetVisibility` (`self.Teddy`) true false)
      (message `/Game/Blueprints/BPI_SleepDeprivedDude.QuestCompleted` _returnvalue "NewEnumerator2"))))

(fn `UserConstructionScript`)