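; Player controller that drives the menu flow between the main menu, World and EndGame levels by checking the current level name.
; On BeginPlay it shows the main menu widget with Game and UI input on MainMenuNEW, or the end game widget on EndGame.
; Space bar on the main menu shows a loading screen, then opens World after a short delay; on EndGame it returns to the main menu.
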(event `Key|SpaceBar`
  (params (Key :type "Key Structure"))
  (:`Pressed`
    (if (== (stale `self.ReceiveBeginPlay` _returnvalue) "MainMenuNEW")
      (bind _returnvalue (`|CreateWidget` "/Game/Widgets/WB_LoadingScreen.WB_LoadingScreen_C"))
      (`UserWidget.AddToViewport` _returnvalue 0)
      (`KismetSystemLibrary.Delay` 0.2)
      (`GameplayStatics.OpenLevel` "World")
      (else
        (bind _returnvalue_2 (`GameplayStatics.GetCurrentLevelName` true))
        (if (== _returnvalue_2 "EndGame")
          (`GameplayStatics.OpenLevel` "MainMenuNEW"))))))

(event `self.ReceiveBeginPlay`
  (`|ExecutionSequence`
    (:`then_0`
      (bind _returnvalue (`GameplayStatics.GetCurrentLevelName` true))
      (if (== _returnvalue "MainMenuNEW")
        (bind _returnvalue_2 (`|CreateWidget` "/Game/Widgets/WB_MainMenu.WB_MainMenu_C"))
        (bind _output_get (set `self.WB_MainMenu` _returnvalue_2))
        (`UserWidget.AddToViewport` _output_get 0)
        (`WidgetBlueprintLibrary.SetInputMode_GameAndUIEx` (`GameplayStatics.GetPlayerController` 0) _output_get)))
    (:`then_1`
      (bind _returnvalue_3 (`GameplayStatics.GetCurrentLevelName` true))
      (if (== _returnvalue_3 "EndGame")
        (bind _returnvalue_4 (`|CreateWidget` "/Game/Widgets/WB_EndGame.WB_EndGame_C"))
        (`UserWidget.AddToViewport` _returnvalue_4 0)))))

(fn `UserConstructionScript`)