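; Tea-making quest station where a player tagged Cup places a cup to brew tea and later picks it up.
; Placing it calls BrewTea on the player, starts kettle audio and spawns a chasing BP_Clown.
; Tick watches the player's brew timer and finished flag to show the pickup prompt and swap boiling for a whistle.
; DoOnce-gated pickup hides the cup, sends the quest interaction and flags the tea stand finished.
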(event `self.ReceiveTick`
  (params (DeltaSeconds :type "Float (single-precision)"))
  (bind _returnvalue (`GameplayStatics.GetPlayerCharacter` 0))
  (bind __bp_sleep_deprived_dude (`self. BP Sleep Deprived Dude`))
  (bind __bp_sleep_deprived_dude_2 (`self. BP Sleep Deprived Dude`))
  (`|ExecutionSequence`
    (:`then_0`
      (if (and (>= (`/Game/Blueprints/BP_SleepDeprivedDude.TeaBrewTimer` __bp_sleep_deprived_dude) (`/Game/Blueprints/BP_SleepDeprivedDude.TeaTimerMax` __bp_sleep_deprived_dude)) (`self.IsOverlapping`))
        (`/Engine/EditorBlueprintResources/StandardMacros.DoOnce` false
          (:`Completed`
            (message `/Game/Blueprints/BPI_Interact.SetPromptText` _returnvalue "Pick up" (`self.Cup`))
            (message `/Game/Blueprints/BPI_Interact.ToggleVisibility` _returnvalue true)))))
    (:`then_1`
      (if (`/Game/Blueprints/BP_SleepDeprivedDude.PlaySoundTeaFinished` __bp_sleep_deprived_dude_2)
        (`/Engine/EditorBlueprintResources/StandardMacros.DoOnce` false
          (:`Completed`
            (set `/Game/Blueprints/BP_SleepDeprivedDude.PlaySoundTeaFinished` false __bp_sleep_deprived_dude_2)
            ;[1 0.9154 0] Peter sound (TeaFinished)
            (`AudioComponent.Stop` (`self.BoilingSound`))
            (`GameplayStatics.PlaySoundAtLocation` "/Game/Sounds/KettleSqueek_Cue.KettleSqueek_Cue" (`SceneComponent.K2_GetComponentLocation` (`self.SoundSpawn`)) (struct) 1.0 1.0 0.0 null null null null)))))))

(event `self.ReceiveBeginPlay`
  (bind _asbp_sleep_deprived_dude (cast `/Game/Blueprints/BP_SleepDeprivedDude` (`GameplayStatics.GetPlayerCharacter` 0)))
  (set `self. BP Sleep Deprived Dude` _asbp_sleep_deprived_dude))

(event `self.QuestDelivery.OnComponentBeginOverlap`
  (params (OverlappedComponent :type "PrimitiveComponent Object Reference") (OtherActor :type "Actor Object Reference") (OtherComp :type "PrimitiveComponent Object Reference") (OtherBodyIndex :type Integer) (bFromSweep :type Boolean) (SweepResult :type "HitResult Structure (by ref)"))
  (bind _returnvalue (`GameplayStatics.GetPlayerCharacter` 0))
  (bind __bp_sleep_deprived_dude (`self. BP Sleep Deprived Dude`))
  (bind _teatime (`/Game/Blueprints/BP_SleepDeprivedDude.TeaTime` (`self. BP Sleep Deprived Dude`)))
  (set `self.IsOverlapping` true)
  (if (== OtherActor _returnvalue)
    (if (`self.ActorHasTag` (`GameplayStatics.GetPlayerCharacter` 0) "Cup")
      (if _teatime
        (if (and (>= (`/Game/Blueprints/BP_SleepDeprivedDude.TeaBrewTimer` __bp_sleep_deprived_dude) (`/Game/Blueprints/BP_SleepDeprivedDude.TeaTimerMax` __bp_sleep_deprived_dude)) (not _teatime)) :!label _label
          (message `/Game/Blueprints/BPI_Interact.SetPromptText` _returnvalue "Pick up" (`self.Cup`))
          (message `/Game/Blueprints/BPI_Interact.ToggleVisibility` _returnvalue true))
        (elif (`self.Block`)
          (goto _label)
          (else
            (message `/Game/Blueprints/BPI_Interact.SetPromptText` _returnvalue "Place" (`self.Cup`))
            (message `/Game/Blueprints/BPI_Interact.ToggleVisibility` _returnvalue true)))))))

(event `self.QuestDelivery.OnComponentEndOverlap`
  (params (OverlappedComponent :type "PrimitiveComponent Object Reference") (OtherActor :type "Actor Object Reference") (OtherComp :type "PrimitiveComponent Object Reference") (OtherBodyIndex :type Integer))
  (set `self.IsOverlapping` false)
  (message `/Game/Blueprints/BPI_Interact.ToggleVisibility` (`GameplayStatics.GetPlayerCharacter` 0) false))

(event `/Game/Blueprints/BPI_Interact.Interact`
  (bind _returnvalue (`GameplayStatics.GetPlayerCharacter` 0))
  (bind (_returnvalue_location _returnvalue_rotation) (`KismetMathLibrary.BreakTransform` (`SceneComponent.K2_GetComponentToWorld` (`self.DemonSpawnPoint`))))
  (if (`self.IsOverlapping`)
    (if (`self.ActorHasTag` (`GameplayStatics.GetPlayerCharacter` 0) "Cup")
      (if (> (`self.Start Index`) 0)
        (if (not (`/Game/Blueprints/BP_SleepDeprivedDude.TeaTime` (`self. BP Sleep Deprived Dude`)))
          (`/Engine/EditorBlueprintResources/StandardMacros.DoOnce` false
            (:`Completed`
              (`GameplayStatics.PlaySoundAtLocation` "/Game/Sounds/PoureTea_Cue.PoureTea_Cue" (`self.K2_GetActorLocation`) (struct) 1.0 1.0 0.0 null null null null)
              (`KismetSystemLibrary.Delay` 2.0)
              (`SceneComponent.SetVisibility` (`self.Cup`) false false)
              (message `/Game/Blueprints/BPI_SleepDeprivedDude.QuestInteraction` _returnvalue "/Game/Assets/QuestAssets/Cup/Cup.Cup" "NewEnumerator0")
              (set `/Game/Blueprints/BP_PlayerTeaStand.TeaIsFinished` true (`self.TeaStandRef`))
              (message `/Game/Blueprints/BPI_Interact.ToggleVisibility` _returnvalue false :!label _label_2))))
        (else
          (`/Engine/EditorBlueprintResources/StandardMacros.DoOnce` false
            (:`Completed`
              (`SceneComponent.SetVisibility` (`self.Cup`) true false)
              (`/Game/Blueprints/BP_SleepDeprivedDude.BrewTea` (`self. BP Sleep Deprived Dude`))
              (set `self.Block` true)
              (`/Engine/EditorBlueprintResources/StandardMacros.IncrementInt` (`self.Start Index`)
                (:`  `
                  ;[1 0.9154 0] Peter sound (Boiling)
                  (bind _returnvalue_2 (`GameplayStatics.SpawnSoundAtLocation` "/Game/Sounds/KettleSound_Cue.KettleSound_Cue" (`SceneComponent.K2_GetComponentLocation` (`self.SoundSpawn`)) (struct) 1.0 1.0 0.0 null null))
                  (set `self.BoilingSound` _returnvalue_2)
                  (bind _returnvalue_3 (`AIBlueprintHelperLibrary.SpawnAIFromClass` "/Game/Blueprints/ScaryBoyJohan/BP_Clown.BP_Clown_C" null (+ _returnvalue_location (0.0 0.0 100.0)) _returnvalue_rotation false null))
                  (bind _asbp_clown (cast `/Game/Blueprints/ScaryBoyJohan/BP_Clown` _returnvalue_3))
                  (set `/Game/Blueprints/ScaryBoyJohan/BP_Clown.ChaseDuration` 35.0 _asbp_clown)
                  (goto _label_2))))))))))

(fn `UserConstructionScript`)