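; BP_QuestItems is an interactable quest pickup whose quest type selects which item it appears as.
; On BeginPlay, it switches on QuestItem to set the QuestMesh to a tea cup, teddy bear, light bulb or sleeping pills, scaling down the teddy.
; Interact passes the mesh and quest type to the player character through QuestInteractionMessage, then destroys the actor.
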(event `self.ReceiveBeginPlay`
  (switch `/Game/Blueprints/E_QuestItems` (`self.QuestItem`)
    (:`NewEnumerator0`
      (`StaticMeshComponent.SetStaticMesh` (`self.QuestMesh`) (`self.TeaCup`)))
    (:`NewEnumerator2`
      (`StaticMeshComponent.SetStaticMesh` (`self.QuestMesh`) (`self.TeddyMesh`))
      (`SceneComponent.SetWorldScale3D` (`self.QuestMesh`) (0.3 0.3 0.3)))
    (:`NewEnumerator3`
      (`StaticMeshComponent.SetStaticMesh` (`self.QuestMesh`) (`self.lightBulbMesh`)))
    (:`NewEnumerator4`
      (`StaticMeshComponent.SetStaticMesh` (`self.QuestMesh`) (`self.SleepingPillsMesh`)))))

(event `/Game/Blueprints/BPI_Interact.Interact`
  (message `/Game/Blueprints/BPI_SleepDeprivedDude.QuestInteraction` (`GameplayStatics.GetPlayerCharacter` 0) (`StaticMeshComponent.StaticMesh` (`self.QuestMesh`)) (`self.QuestItem`))
  (`self.K2_DestroyActor`))

(fn `Teddy Mesh`
  (params (NewMesh :type "StaticMesh Object Reference"))
  (`StaticMeshComponent.SetStaticMesh` (`self.QuestMesh`) NewMesh))

(fn `UserConstructionScript`)