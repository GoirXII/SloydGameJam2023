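; BP_Door is an interactive door that shows the player an "Open" prompt inside its box trigger and swings on Interact.
; Interact checks open, moving and overlap flags, then runs open or close timelines that rotate the door's yaw, with DoOnce-gated hinge sounds.
; A separate DoorSlam event plays a slam-shut timeline and sound for jumpscares.
; The construction script picks one of two glass materials from HasGlassInDoor.
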(event `/Game/Blueprints/BPI_Interact.Interact`
  ;[1 1 1] interaction
  (if (`self.CanOpen`)
    (if (`self.CurrentlMoving`)
      _
      (elif (and (`self.IsOpen`) (`self.IsOverlapping`))
        (`self.Close Door`)
        (else
          ;;[1 0.8075 0] sound
          (`GameplayStatics.PlaySoundAtLocation` "/Game/Sounds/DoorSounds/DoorOpen2_Cue.DoorOpen2_Cue" (`SceneComponent.RelativeLocation` (`self.HingeNoiseLocation`)) (struct) 1.0 1.0 0.0 null null null null)
          (set `self.CurrentlMoving` true)
          (`self.Open Door`))))))

(event `Open Door`
  ;[1 1 1] Door OpenClose
  (set `self.CurrentlMoving` true)
  (bind (_direction _movement) (`Timeline|DoorMovement` :!via `PlayFromStart`)
    (:`Update`
      (`SceneComponent.K2_SetRelativeRotation` (`self.Door`) (`KismetMathLibrary.MakeRotator` 0.0 0.0 (* _movement 90.0)) false false)
      (`/Engine/EditorBlueprintResources/StandardMacros.DoOnce` false :!label _label
        (:`Completed`
          ;;[1 0.8189 0] squeaking noise
          (`GameplayStatics.PlaySoundAtLocation` "/Game/Sounds/DoorSounds/DoorSqueak_Cue.DoorSqueak_Cue" (`SceneComponent.RelativeLocation` (`self.HingeNoiseLocation`)) (struct) 1.0 1.0 0.0 null null null null))))
    (:`Finished`
      (set `self.IsOpen` true)
      (set `self.CurrentlMoving` false)
      (goto _label :!via `Reset`))))

(event `Close Door`
  ;[1 1 1] Door OpenClose
  (set `self.CurrentlMoving` true)
  (bind (_direction _movement _movementclosed) (`Timeline|Timeline` :!via `PlayFromStart`)
    (:`Update`
      (`SceneComponent.K2_SetRelativeRotation` (`self.Door`) (`KismetMathLibrary.MakeRotator` 0.0 0.0 (* _movementclosed 90.0)) false false)
      (`/Engine/EditorBlueprintResources/StandardMacros.DoOnce` false :!label _label_2
        (:`Completed`
          ;;[1 0.8724 0] squaking noise
          (`GameplayStatics.PlaySoundAtLocation` "/Game/Sounds/DoorSounds/DoorSqueak_Cue.DoorSqueak_Cue" (`SceneComponent.RelativeLocation` (`self.HingeNoiseLocation`)) (struct) 1.0 1.0 0.0 null null null null)
          ;;[1 0.9505 0] close sound
          (`GameplayStatics.PlaySoundAtLocation` "/Game/Sounds/DoorSounds/DoorClose_Cue.DoorClose_Cue" (`SceneComponent.RelativeLocation` (`self.HingeNoiseLocation`)) (struct) 1.0 1.0 0.0 null null null null))))
    (:`Finished`
      (set `self.IsOpen` false)
      (set `self.CurrentlMoving` false)
      (goto _label_2 :!via `Reset`))))

(event `/Game/Blueprints/BPI_Interact.DoorSlam`
  ;[1 1 1] door effect if jumpscared
  (set `self.CurrentlMoving` false)
  (bind (_direction _movement _movementclosed) (`Timeline|Timeline_0` :!via `PlayFromStart`)
    (:`Update`
      (`SceneComponent.K2_SetRelativeRotation` (`self.Door`) (`KismetMathLibrary.MakeRotator` 0.0 0.0 (* _movementclosed 90.0)) false false)
      (`/Engine/EditorBlueprintResources/StandardMacros.DoOnce` false :!label _label_3
        (:`Completed`
          ;[1 0.7811 0] close sound
          (`GameplayStatics.PlaySoundAtLocation` "/Game/Sounds/DoorSounds/DoorSlam_Cue1.DoorSlam_Cue1" (`SceneComponent.RelativeLocation` (`self.HingeNoiseLocation`)) (struct) 1.0 1.0 0.0 null null null null))))
    (:`Finished`
      (set `self.IsOpen` false)
      (goto _label_3 :!via `Reset`))))

(event `self.Box.OnComponentBeginOverlap`
  (params (OverlappedComponent :type "PrimitiveComponent Object Reference") (OtherActor :type "Actor Object Reference") (OtherComp :type "PrimitiveComponent Object Reference") (OtherBodyIndex :type Integer) (bFromSweep :type Boolean) (SweepResult :type "HitResult Structure (by ref)"))
  (bind _returnvalue (`GameplayStatics.GetPlayerCharacter` 0))
  (if (`self.CanOpen`)
    (if (== OtherActor _returnvalue)
      (bind _output_get (set `self.IsOverlapping` true))
      (message `/Game/Blueprints/BPI_Interact.SetPromptText` _returnvalue "Open" (`self.Door`))
      (message `/Game/Blueprints/BPI_Interact.ToggleVisibility` _returnvalue _output_get))))

(event `self.Box.OnComponentEndOverlap`
  (params (OverlappedComponent :type "PrimitiveComponent Object Reference") (OtherActor :type "Actor Object Reference") (OtherComp :type "PrimitiveComponent Object Reference") (OtherBodyIndex :type Integer))
  (if (`self.CanOpen`)
    (bind _output_get (set `self.IsOverlapping` false))
    (message `/Game/Blueprints/BPI_Interact.ToggleVisibility` (`GameplayStatics.GetPlayerCharacter` 0) _output_get)))

(fn `UserConstructionScript`
  (if (`self.HasGlassInDoor`)
    (`PrimitiveComponent.SetMaterial` (`self.Door`) 1 "/Game/Assets/Door/M_Glass.M_Glass")
    (else
      (`PrimitiveComponent.SetMaterial` (`self.Door`) 1 "/Game/Assets/Door/M_Glass2.M_Glass2"))))