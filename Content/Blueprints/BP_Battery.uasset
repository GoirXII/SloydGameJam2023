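; BP_Battery is a battery pickup that passes its BatteryCharge to the player character when interacted with.
; Its Sphere overlap toggles a "Pick up" prompt on the player character, with only the begin overlap checking that the other actor is the player.
; The Interact event plays a sound at the battery's location, sends the charge through UpdateBatteryLifeMessage, then destroys the actor.
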(event `/Game/Blueprints/BPI_Interact.Interact`
  ;[1 1 1] play sound to change battery
  (`GameplayStatics.PlaySoundAtLocation` "/Game/Sounds/BatteryLow_Cue.BatteryLow_Cue" (`self.K2_GetActorLocation`) (struct) 1.0 1.0 0.0 null null null null)
  (message `/Game/Blueprints/BPI_Interact.UpdateBatteryLife` (`GameplayStatics.GetPlayerCharacter` 0) (`self.BatteryCharge`))
  (`self.K2_DestroyActor`))

(event `self.Sphere.OnComponentBeginOverlap`
  (params (OverlappedComponent :type "PrimitiveComponent Object Reference") (OtherActor :type "Actor Object Reference") (OtherComp :type "PrimitiveComponent Object Reference") (OtherBodyIndex :type Integer) (bFromSweep :type Boolean) (SweepResult :type "HitResult Structure (by ref)"))
  (bind _returnvalue (`GameplayStatics.GetPlayerCharacter` 0))
  (if (== OtherActor _returnvalue)
    (bind _output_get (set `self.IsOverlapping` true))
    (message `/Game/Blueprints/BPI_Interact.SetPromptText` _returnvalue "Pick up" (`self.Battery`))
    (message `/Game/Blueprints/BPI_Interact.ToggleVisibility` _returnvalue _output_get)))

(event `self.Sphere.OnComponentEndOverlap`
  (params (OverlappedComponent :type "PrimitiveComponent Object Reference") (OtherActor :type "Actor Object Reference") (OtherComp :type "PrimitiveComponent Object Reference") (OtherBodyIndex :type Integer))
  (bind _output_get (set `self.IsOverlapping` false))
  (message `/Game/Blueprints/BPI_Interact.ToggleVisibility` (`GameplayStatics.GetPlayerCharacter` 0) _output_get))

(fn `UserConstructionScript`)