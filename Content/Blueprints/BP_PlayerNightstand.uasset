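; BP_PlayerNightstand is a nightstand that serves as the drop-off point for a pills delivery quest.
; Overlapping its QuestDelivery component shows a "Place" prompt if the player has the "Pills" tag, and leaving hides it.
; Interact rechecks overlap and tag, then reveals the Pills component, reports quest completion to the player character and hides the prompt.
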(event `self.QuestDelivery.OnComponentBeginOverlap`
  (params (OverlappedComponent :type "PrimitiveComponent Object Reference") (OtherActor :type "Actor Object Reference") (OtherComp :type "PrimitiveComponent Object Reference") (OtherBodyIndex :type Integer) (bFromSweep :type Boolean) (SweepResult :type "HitResult Structure (by ref)"))
  (bind _returnvalue (`GameplayStatics.GetPlayerCharacter` 0))
  (if (== OtherActor _returnvalue)
    (if (`self.ActorHasTag` (`GameplayStatics.GetPlayerCharacter` 0) "Pills")
      (set `self.IsOverlapping` true)
      (message `/Game/Blueprints/BPI_Interact.SetPromptText` _returnvalue "Place" (`self.Pills`))
      (message `/Game/Blueprints/BPI_Interact.ToggleVisibility` _returnvalue true))))

(event `self.QuestDelivery.OnComponentEndOverlap`
  (params (OverlappedComponent :type "PrimitiveComponent Object Reference") (OtherActor :type "Actor Object Reference") (OtherComp :type "PrimitiveComponent Object Reference") (OtherBodyIndex :type Integer))
  (set `self.IsOverlapping` false)
  (message `/Game/Blueprints/BPI_Interact.ToggleVisibility` (`GameplayStatics.GetPlayerCharacter` 0) false))

(event `/Game/Blueprints/BPI_Interact.Interact`
  (bind _returnvalue (`GameplayStatics.GetPlayerCharacter` 0))
  (if (`self.IsOverlapping`)
    (if (`self.ActorHasTag` _returnvalue "Pills")
      (`SceneComponent.SetVisibility` (`self.Pills`) true false)
      (message `/Game/Blueprints/BPI_SleepDeprivedDude.QuestCompleted` _returnvalue "NewEnumerator4")
      (message `/Game/Blueprints/BPI_Interact.ToggleVisibility` _returnvalue false))))

(fn `UserConstructionScript`)