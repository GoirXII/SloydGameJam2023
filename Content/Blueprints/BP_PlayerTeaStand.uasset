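; BP_PlayerTeaStand is a quest delivery spot where the player places a finished cup of tea.
; The QuestDelivery overlap shows a "Place" prompt when the player carries the Cup tag and TeaIsFinished is set, and hides it on exit.
; Interact rechecks those conditions, reveals the stand's Cup component, reports the quest completed and hides the prompt, messaging the player character through interface calls.
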(event `self.QuestDelivery.OnComponentBeginOverlap`
  (params (OverlappedComponent :type "PrimitiveComponent Object Reference") (OtherActor :type "Actor Object Reference") (OtherComp :type "PrimitiveComponent Object Reference") (OtherBodyIndex :type Integer) (bFromSweep :type Boolean) (SweepResult :type "HitResult Structure (by ref)"))
  (bind _returnvalue (`GameplayStatics.GetPlayerCharacter` 0))
  (set `self.IsOverlapping` true)
  (if (== OtherActor _returnvalue)
    (if (`self.ActorHasTag` (`GameplayStatics.GetPlayerCharacter` 0) "Cup")
      (if (`self.TeaIsFinished`)
        (message `/Game/Blueprints/BPI_Interact.SetPromptText` _returnvalue "Place" (`self.Cup`))
        (message `/Game/Blueprints/BPI_Interact.ToggleVisibility` _returnvalue false)))))

(event `self.QuestDelivery.OnComponentEndOverlap`
  (params (OverlappedComponent :type "PrimitiveComponent Object Reference") (OtherActor :type "Actor Object Reference") (OtherComp :type "PrimitiveComponent Object Reference") (OtherBodyIndex :type Integer))
  (bind _output_get (set `self.IsOverlapping` false))
  (message `/Game/Blueprints/BPI_Interact.ToggleVisibility` (`GameplayStatics.GetPlayerCharacter` 0) _output_get))

(event `/Game/Blueprints/BPI_Interact.Interact`
  (bind _returnvalue (`GameplayStatics.GetPlayerCharacter` 0))
  (if (and (`self.IsOverlapping`) (`self.TeaIsFinished`))
    (if (`self.ActorHasTag` _returnvalue "Cup")
      (`SceneComponent.SetVisibility` (`self.Cup`) true false)
      (message `/Game/Blueprints/BPI_SleepDeprivedDude.QuestCompleted` _returnvalue "NewEnumerator0")
      (message `/Game/Blueprints/BPI_Interact.ToggleVisibility` _returnvalue false))))

(fn `UserConstructionScript`)