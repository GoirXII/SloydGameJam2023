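; BP_PlayerLamp is a lamp that serves as the delivery point for a light bulb quest.
; Overlapping the QuestDelivery volume shows a "Place" prompt if the player carries the LightBulb tag.
; Interacting inside it with that tag plays a screwing sound, reveals the bulb mesh and reports the quest completed to the player.
; The point light's intensity is raised after a short delay.
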(event `self.QuestDelivery.OnComponentBeginOverlap`
  (params (OverlappedComponent :type "PrimitiveComponent Object Reference") (OtherActor :type "Actor Object Reference") (OtherComp :type "PrimitiveComponent Object Reference") (OtherBodyIndex :type Integer) (bFromSweep :type Boolean) (SweepResult :type "HitResult Structure (by ref)"))
  (bind _returnvalue (`GameplayStatics.GetPlayerCharacter` 0))
  (set `self.IsOverlapping` true)
  (if (== OtherActor _returnvalue)
    (if (`self.ActorHasTag` (`GameplayStatics.GetPlayerCharacter` 0) "LightBulb")
      (message `/Game/Blueprints/BPI_Interact.SetPromptText` _returnvalue "Place" (`self.LightBulb`))
      (message `/Game/Blueprints/BPI_Interact.ToggleVisibility` _returnvalue true))))

(event `self.QuestDelivery.OnComponentEndOverlap`
  (params (OverlappedComponent :type "PrimitiveComponent Object Reference") (OtherActor :type "Actor Object Reference") (OtherComp :type "PrimitiveComponent Object Reference") (OtherBodyIndex :type Integer))
  (set `self.IsOverlapping` false)
  (message `/Game/Blueprints/BPI_Interact.ToggleVisibility` (`GameplayStatics.GetPlayerCharacter` 0) false))

(event `/Game/Blueprints/BPI_Interact.Interact`
  (bind _returnvalue (`GameplayStatics.GetPlayerCharacter` 0))
  (if (`self.IsOverlapping`)
    (if (`self.ActorHasTag` _returnvalue "LightBulb")
      ;[1 0.8366 0] lightbulb sound
      (`GameplayStatics.PlaySoundAtLocation` "/Game/Sounds/LightBulbScrewing_Cue.LightBulbScrewing_Cue" (`self.K2_GetActorLocation`) (struct) 1.0 1.0 0.0 null null null null)
      (`SceneComponent.SetVisibility` (`self.LightBulb`) true false)
      (message `/Game/Blueprints/BPI_SleepDeprivedDude.QuestCompleted` _returnvalue "NewEnumerator3")
      (message `/Game/Blueprints/BPI_Interact.ToggleVisibility` _returnvalue false)
      (`KismetSystemLibrary.Delay` 2.0)
      (`LightComponent.SetIntensity` (`self.PointLight`) 3.0))))

(fn `UserConstructionScript`)